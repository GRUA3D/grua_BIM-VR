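; VR player controller that handles walking, turning and menu interaction for the player character in an architectural model.
; On BeginPlay with a headset enabled, it sets eye-level tracking, pixel density and the VR navigation Enhanced Input context.
; Movement inputs use only the axis sign, applying fixed scales along camera vectors received through the VectoresCamara event.
; Rotation input yaws the character, and releasing the right trigger sends it a menu interaction message.
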(event `self.ReceiveBeginPlay`
  ;[1 0.6527 0.1765] Captura del mapeo de contexto de entrada
  (`|ExecutionSequence`
    (:`then_0`
      (if (`HeadMountedDisplayFunctionLibrary.IsHeadMountedDisplayEnabled`)
        (`HeadMountedDisplayFunctionLibrary.SetTrackingOrigin` "Eye")
        (`KismetSystemLibrary.ExecuteConsoleCommand` "vr.PixelDensity 1.0" null)
        (`EnhancedInputSubsystemInterface.AddMappingContext` (pcsubsystem `EnhancedInputLocalPlayerSubsystem` self) "/Game/Modelo_ARQ/Inputs/IMC_Navegacion_VR.IMC_Navegacion_VR" 0 (struct))))))

(event `EnhancedInput|/Game/Modelo_ARQ/Inputs/IA_Movimiento_X`
  (params (ActionValue :type "Float (double-precision)") (ElapsedSeconds :type "Float (double-precision)") (TriggeredSeconds :type "Float (double-precision)") (InputAction :type "InputAction Object Reference" :default "/Game/Modelo_ARQ/Inputs/IA_Movimiento_X.IA_Movimiento_X"))
  (bind _returnvalue (`GameplayStatics.GetPlayerCharacter` 0))
  ;[0.1995 0.534 1] Navegacion personaje
  (:`Triggered`
    (if (> ActionValue 0.0)
      (`Pawn.AddMovementInput` _returnvalue (stale `/Game/Modelo_ARQ/Blueprint/BI_VectoresCamara.VectoresCamara` RightVector) 0.2 false)
      (else
        (`Pawn.AddMovementInput` _returnvalue (* (stale `/Game/Modelo_ARQ/Blueprint/BI_VectoresCamara.VectoresCamara` RightVector) -1.0) 0.2 false)))))

(event `/Game/Modelo_ARQ/Blueprint/BI_VectoresCamara.VectoresCamara`
  (params (RightVector :type "Vector Structure") (ForwardVector :type "Vector Structure"))
  ;[0.1995 0.534 1] Navegacion personaje
)

(event `EnhancedInput|/Game/Modelo_ARQ/Inputs/IA_Movimiento_Y`
  (params (ActionValue :type "Float (double-precision)") (ElapsedSeconds :type "Float (double-precision)") (TriggeredSeconds :type "Float (double-precision)") (InputAction :type "InputAction Object Reference" :default "/Game/Modelo_ARQ/Inputs/IA_Movimiento_Y.IA_Movimiento_Y"))
  (bind _returnvalue (`GameplayStatics.GetPlayerCharacter` 0))
  ;[0.1995 0.534 1] Navegacion personaje
  (:`Triggered`
    (if (< ActionValue 0.0)
      (`Pawn.AddMovementInput` _returnvalue (* (stale `/Game/Modelo_ARQ/Blueprint/BI_VectoresCamara.VectoresCamara` ForwardVector) -1.0) 0.4 false)
      (else
        (`Pawn.AddMovementInput` _returnvalue (stale `/Game/Modelo_ARQ/Blueprint/BI_VectoresCamara.VectoresCamara` ForwardVector) 0.4 false)))))

(event `EnhancedInput|/Game/Modelo_ARQ/Inputs/IA_Rotacion_Z`
  (params (ActionValue :type "Float (double-precision)") (ElapsedSeconds :type "Float (double-precision)") (TriggeredSeconds :type "Float (double-precision)") (InputAction :type "InputAction Object Reference" :default "/Game/Modelo_ARQ/Inputs/IA_Rotacion_Z.IA_Rotacion_Z"))
  ;[0.1995 0.534 1] Navegacion personaje
  (:`Triggered`
    (`self.K2_AddActorLocalRotation` (`GameplayStatics.GetPlayerCharacter` 0) (`KismetMathLibrary.MakeRotator` 0.0 0.0 (* ActionValue 3.0)) false false)))

(event `EnhancedInput|/Game/Modelo_ARQ/Inputs/IA_Disparo_R`
  (params (ActionValue :type Boolean) (ElapsedSeconds :type "Float (double-precision)") (TriggeredSeconds :type "Float (double-precision)") (InputAction :type "InputAction Object Reference" :default "/Game/Modelo_ARQ/Inputs/IA_Disparo_R.IA_Disparo_R"))
  (:`Completed`
    (message `/Game/Modelo_ARQ/Blueprint/BI_WidgetInteraction.InteraccionMenu` (`GameplayStatics.GetPlayerCharacter` 0) false)))

(fn `UserConstructionScript`)