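; VR player Blueprint for exploring a rural-house BIM model with Niagara laser pointers and a widget menu.
; The menu appears when the camera and an arrow component face each other, and switches between measurement, 4D simulation, selection and filter modes.
; A data table links rows to tagged actors, driving timed construction reveal and category visibility.
; Measurement spawns dimensions between traced points; selection spawns a material plane keyed by assembly code.
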(event `self.ReceiveTick`
  (params (DeltaSeconds :type "Float (single-precision)"))
  (bind _camera (`self.Camera`))
  (bind _w_menu (`self.W_Menu`))
  ;[0.3787 1 0.6401] Vectores Camara
  (`|ExecutionSequence`
    (:`then_0`
      (message `/Game/Modelo_ARQ/Blueprint/BI_VectoresCamara.VectoresCamara` (`GameplayStatics.GetPlayerController` 0) (stale _output_get) (stale _output_get_2)))
    (:`then_1`
      (bind _output_get (set `self.CamaraR` (`SceneComponent.GetRightVector` _camera))))
    (:`then_2`
      (bind _output_get_2 (set `self.CamaraF` (`SceneComponent.GetForwardVector` _camera))))
    (:`then_3`
      (`self.TimerClock`))
    (:`then_4`
      (`self.Filtro`))
    (:`then_5`
      ;[1 1 1] Visibilidad Menu principal
      (bind _returnvalue (`self.Activa_Menu`))
      (if _returnvalue
        (`SceneComponent.SetVisibility` _w_menu true false)
        (set `WidgetInteractionComponent.DebugColor` (`KismetMathLibrary.MakeColor` 0.192708 0.533181 1.0) (`self.WidgetInteraction_R`))
        (else
          (`SceneComponent.SetVisibility` _w_menu false false)
          (set `WidgetInteractionComponent.DebugColor` (`KismetMathLibrary.MakeColor` 1.0) (`self.WidgetInteraction_R`)))))))

(event `self.ReceiveBeginPlay`
  ;[1 1 1] ELEMENTOS INICIALES
  (`self.Punteros_Motion`)
  (`KismetSystemLibrary.K2_SetTimerDelegate` (`|CreateDelegate` :!event `AlcanceLaser_R`) 0.01 true)
  (`KismetSystemLibrary.K2_SetTimerDelegate` (`|CreateDelegate` :!event `AlcanceLaser_L`) 0.01 true))

(event `Retorno_Menu2`
  ;[0.2958 0.9102 1] Menu Interacción
  (bind _returnvalue (`|CreateWidget` "/Game/Modelo_ARQ/Interfaz/UI_Menu_Level2.UI_Menu_Level2_C"))
  (`WidgetComponent.SetWidget` (`self.W_Menu`) _returnvalue)
  (set `self.M_Medicion` false)
  (set `self.M_4D` false)
  (set `self.M_Seleccion` false)
  (set `self.M_Filtro` false)
  (`self.LimpiarMedicion`)
  (bind _outrownames (`DataTableFunctionLibrary.GetDataTableRowNames` "/Game/Modelo_ARQ/DataProject/ParametrosModelo-CasaRural_Feb.ParametrosModelo-CasaRural_Feb"))
  (for _index (range (`KismetArrayLibrary.Array_Length` _outrownames))
    (`self.Hidden/Visible` false _index)
    (bind _returnvalue_2 (`GameplayStatics.GetActorOfClass` "/Game/Modelo_ARQ/Especificaciones/MP_Plane.MP_Plane_C"))
    (`/Engine/EditorBlueprintResources/StandardMacros.IsValid` _returnvalue_2
      (:`Is Valid`
        (`self.K2_DestroyActor`)))))

(event `Retorno_Menu`
  ;[0.2958 0.9102 1] Menu Interacción
  (bind _returnvalue (`|CreateWidget` "/Game/Modelo_ARQ/Interfaz/UI_Menu_Inicial.UI_Menu_Inicial_C"))
  (`WidgetComponent.SetWidget` (`self.W_Menu`) _returnvalue))

(event `4D_On`
  ;[0.2958 0.9102 1] Menu Interacción
  (bind _returnvalue (`|CreateWidget` "/Game/Modelo_ARQ/Interfaz/UI_Menu_Bim4D.UI_Menu_Bim4D_C"))
  (`WidgetComponent.SetWidget` (`self.W_Menu`) _returnvalue)
  (set `self.M_4D` true)
  (`self.4D_Modo_iniciar`))

(event `Medicion_On`
  ;[0.2958 0.9102 1] Menu Interacción
  (bind _returnvalue (`|CreateWidget` "/Game/Modelo_ARQ/Interfaz/UI_Menu_medicion.UI_Menu_medicion_C"))
  (`WidgetComponent.SetWidget` (`self.W_Menu`) _returnvalue)
  (set `self.M_Medicion` true))

(event `/Game/Modelo_ARQ/Blueprint/BI_WidgetInteraction.MenuModo`
  (params (ActivarModo :type Boolean) (Retorno_menu :type Boolean) (Medicion_ON :type Boolean) (`4D_ON` :type Boolean) (Filtro_ON :type Boolean) (Retorno_menu_2 :type Boolean) (Seleccion_ON :type Boolean))
  ;[0.2958 0.9102 1] Menu Interacción
  (`|ExecutionSequence`
    (:`then_0`
      (if (or ActivarModo Retorno_menu_2)
        (`self.Retorno_Menu2`)))
    (:`then_1`
      (if Retorno_menu
        (`self.Retorno_Menu`)))
    (:`then_2`
      (if Medicion_ON
        (`self.Medicion_On`)))
    (:`then_3`
      (if `4D_ON`
        (`self.4D_On`)))
    (:`then_4`
      (if Seleccion_ON
        (`self.Seleccion_On`)))
    (:`then_5`
      (if Filtro_ON
        (`self.Filtro_On`)))))

(event `Seleccion_On`
  ;[0.2958 0.9102 1] Menu Interacción
  (bind _returnvalue (`|CreateWidget` "/Game/Modelo_ARQ/Interfaz/UI_Menu_Seleccion.UI_Menu_Seleccion_C"))
  (`WidgetComponent.SetWidget` (`self.W_Menu`) _returnvalue)
  (set `self.M_Seleccion` true))

(event `Filtro_On`
  ;[0.2958 0.9102 1] Menu Interacción
  (bind _returnvalue (`|CreateWidget` "/Game/Modelo_ARQ/Interfaz/UI_Menu_Filtros1.UI_Menu_Filtros1_C"))
  (`WidgetComponent.SetWidget` (`self.W_Menu`) _returnvalue)
  (set `self.M_Filtro` true))

(event `Punteros_Motion`
  ;[0.3927 1 0.2087] Asignacion de distancia apuntador
  (bind _returnvalue (`NiagaraFunctionLibrary.SpawnSystemAttached` "/Game/Modelo_ARQ/Interfaz/NS_Laser.NS_Laser" (`self.MotionController_R`) "None" (0.0 0.0 0.0) (struct :`Pitch` 290.0) "KeepRelativeOffset"))
  (set `self.Point_R` _returnvalue)
  (bind _returnvalue_2 (`NiagaraFunctionLibrary.SpawnSystemAttached` "/Game/Modelo_ARQ/Interfaz/NS_Laser.NS_Laser" (`self.MotionController_L`) "None" (0.0 0.0 0.0) (struct :`Pitch` 290.0) "KeepRelativeOffset"))
  (set `self.Point_L` _returnvalue_2))

(event `/Game/Modelo_ARQ/Blueprint/BI_WidgetInteraction.InteraccionMenu`
  (params (Menu :type Boolean))
  (bind _widgetinteraction_r (`self.WidgetInteraction_R`))
  ;[0.2958 0.9102 1] Menu Interacción
  (`|ExecutionSequence`
    (:`then_0`
      (`WidgetInteractionComponent.PressPointerKey` _widgetinteraction_r "LeftMouseButton"))
    (:`then_1`
      (`WidgetInteractionComponent.ReleasePointerKey` _widgetinteraction_r "LeftMouseButton"))))

(event `EnhancedInput|/Game/Modelo_ARQ/Inputs/IA_Scroll_Y`
  (params (ActionValue :type "Float (double-precision)") (ElapsedSeconds :type "Float (double-precision)") (TriggeredSeconds :type "Float (double-precision)") (InputAction :type "InputAction Object Reference" :default "/Game/Modelo_ARQ/Inputs/IA_Scroll_Y.IA_Scroll_Y"))
  ;[0.2958 0.9102 1] Menu Interacción
  (:`Triggered`
    (`WidgetInteractionComponent.ScrollWheel` (`self.WidgetInteraction_R`) (* ActionValue 0.25))))

(event `AlcanceLaser_R`
  (bind _bp_por (`self.BP_PoR`))
  (bind _bp_por_2 (`self.BP_PoR`))
  (bind _point_r (`self.Point_R`))
  ;[0.3927 1 0.2087] Asignacion de distancia apuntador
  (`/Engine/EditorBlueprintResources/StandardMacros.IsValid` _point_r
    (:`Is Valid`
      (bind (_start _end _hitevent) (`self.TrazadoApuntador` (`self.MotionController_R`)))
      (`SceneComponent.K2_SetRelativeLocationAndRotation` (`self.WidgetInteraction_R`) (0.0 0.0 0.0) (struct :`Pitch` 290.0) false false)
      (bind (_bblockinghit _binitialoverlap _time _distance _location _impactpoint) (`GameplayStatics.BreakHitResult` _hitevent))
      (if _bblockinghit
        (`NiagaraComponent.SetVariableVec3` _point_r "Laser End" (`KismetMathLibrary.MakeVector` _distance))
        (`/Engine/EditorBlueprintResources/StandardMacros.IsValid` _bp_por
          (:`Is Valid`
            (`self.K2_SetActorLocation` _bp_por _impactpoint false false))
          (:`Is Not Valid`
            (`self.PointR`)))
        (else
          (`NiagaraComponent.SetVariableVec3` _point_r "Laser End" (`KismetMathLibrary.MakeVector` (`KismetMathLibrary.Vector_Distance` _start _end)))
          (`/Engine/EditorBlueprintResources/StandardMacros.IsValid` _bp_por_2
            (:`Is Valid`
              (`self.K2_DestroyActor` _bp_por_2))))))))

(event `AlcanceLaser_L`
  (bind _point_l (`self.Point_L`))
  (bind _bp_pol (`self.BP_PoL`))
  (bind _bp_pol_2 (`self.BP_PoL`))
  ;[0.3927 1 0.2087] Asignacion de distancia apuntador
  (`/Engine/EditorBlueprintResources/StandardMacros.IsValid` _point_l
    (:`Is Valid`
      (bind (_start _end _hitevent) (`self.TrazadoApuntador` (`self.MotionController_L`)))
      (`SceneComponent.K2_SetRelativeLocationAndRotation` (`self.WidgetInteraction_L`) (0.0 0.0 0.0) (struct :`Pitch` 290.0) false false)
      (bind (_bblockinghit _binitialoverlap _time _distance _location _impactpoint) (`GameplayStatics.BreakHitResult` _hitevent))
      (if _bblockinghit
        (`NiagaraComponent.SetVariableVec3` _point_l "Laser End" (`KismetMathLibrary.MakeVector` _distance))
        (`/Engine/EditorBlueprintResources/StandardMacros.IsValid` _bp_pol_2
          (:`Is Valid`
            (`self.K2_SetActorLocation` _bp_pol_2 _impactpoint false false))
          (:`Is Not Valid`
            (`self.PointL`)))
        (else
          (`NiagaraComponent.SetVariableVec3` _point_l "Laser End" (`KismetMathLibrary.MakeVector` (`KismetMathLibrary.Vector_Distance` _start _end)))
          (`/Engine/EditorBlueprintResources/StandardMacros.IsValid` _bp_pol
            (:`Is Valid`
              (`self.K2_DestroyActor` _bp_pol))))))))

(event `PointR`
  (bind _point_r (`self.Point_R`))
  ;[0.3927 1 0.2087] Asignacion de distancia apuntador
  (`/Engine/EditorBlueprintResources/StandardMacros.IsValid` _point_r
    (:`Is Valid`
      (bind _returnvalue (`|SpawnActorFromClass` "/Game/Modelo_ARQ/Blueprint/BP_Pointer.BP_Pointer_C" (`KismetMathLibrary.MakeTransform` (`SceneComponent.K2_GetComponentLocation` _point_r) (struct) (0.4 0.4 0.4)) "AlwaysSpawn" "MultiplyWithRoot" null self))
      (set `self.BP_PoR` _returnvalue))))

(event `PointL`
  (bind _point_l (`self.Point_L`))
  ;[0.3927 1 0.2087] Asignacion de distancia apuntador
  (`/Engine/EditorBlueprintResources/StandardMacros.IsValid` _point_l
    (:`Is Valid`
      (bind _returnvalue (`|SpawnActorFromClass` "/Game/Modelo_ARQ/Blueprint/BP_Pointer.BP_Pointer_C" (`KismetMathLibrary.MakeTransform` (`SceneComponent.K2_GetComponentLocation` _point_l) (struct) (0.4 0.4 0.4)) "Undefined" "MultiplyWithRoot" null self))
      (set `self.BP_PoL` _returnvalue))))

(event `EnhancedInput|/Game/Modelo_ARQ/Inputs/IA_Disparo_R`
  (params (ActionValue :type Boolean) (ElapsedSeconds :type "Float (double-precision)") (TriggeredSeconds :type "Float (double-precision)") (InputAction :type "InputAction Object Reference" :default "/Game/Modelo_ARQ/Inputs/IA_Disparo_R.IA_Disparo_R"))
  ;[0.9819 0.2169 1] Modo Medicion
  (:`Started`
    (if (and (`self.M_Medicion`) ActionValue)
      (bind (_start _end _hitevent) (`self.TrazadoApuntador` (`self.MotionController_R`)))
      (bind (_bblockinghit _binitialoverlap _time _distance _location _impactpoint) (`GameplayStatics.BreakHitResult` _hitevent))
      (if _bblockinghit
        (if (== (`self.M_MedContador`) 0)
          (set `self.M_MedContador` 1))
        (if (== (`self.M_MedContador`) 1)
          (set `self.M_MedPoint A` _impactpoint)
          (set `self.M_MedContador` 2)
          (`KismetSystemLibrary.Delay` 5.0)
          (set `self.M_MedContador` 0)
          (elif (== (`self.M_MedContador`) 2)
            (set `self.M_MedPoint B` _impactpoint)
            (set `self.M_MedContador` 0)
            (`|SpawnActorFromClass` :`Class` "/Game/CollaborativeViewer/Blueprints/Commands/Dimension/BPs/BP_Dimenssion.BP_Dimenssion_C" :`SpawnTransform` (`KismetMathLibrary.MakeTransform` (0.0 0.0 0.0)) :`CollisionHandlingOverride` "Undefined" :`TransformScaleMethod` "MultiplyWithRoot" :`PointA` (`self.M_MedPoint A`) :`PointB` (`self.M_MedPoint B`) :`Instigator` null :!label _label)))
        (else
          (set `self.M_MedContador` 0))))))

(event `EnhancedInput|/Game/Modelo_ARQ/Inputs/IA_Disparo_L`
  (params (ActionValue :type Boolean) (ElapsedSeconds :type "Float (double-precision)") (TriggeredSeconds :type "Float (double-precision)") (InputAction :type "InputAction Object Reference" :default "/Game/Modelo_ARQ/Inputs/IA_Disparo_L.IA_Disparo_L"))
  ;[0.9819 0.2169 1] Modo Medicion
  (:`Started`
    (if (and ActionValue (`self.M_Medicion`))
      (bind (_start _end _hitevent) (`self.TrazadoApuntador` (`self.MotionController_L`)))
      (bind (_bblockinghit _binitialoverlap _time _distance _location _impactpoint) (`GameplayStatics.BreakHitResult` _hitevent))
      (if _bblockinghit
        (if (== (`self.M_MedContador`) 0)
          (set `self.M_MedContador` 1))
        (if (== (`self.M_MedContador`) 1)
          (set `self.M_MedPoint A` _impactpoint)
          (set `self.M_MedContador` 2)
          (`KismetSystemLibrary.Delay` 10.0)
          (set `self.M_MedContador` 0)
          (elif (== (`self.M_MedContador`) 2)
            (set `self.M_MedPoint B` _impactpoint)
            (set `self.M_MedContador` 0)
            (goto _label)))
        (else
          (set `self.M_MedContador` 0))))))

(event `EnhancedInput|/Game/Modelo_ARQ/Inputs/IA_Boton_X`
  (params (ActionValue :type Boolean) (ElapsedSeconds :type "Float (double-precision)") (TriggeredSeconds :type "Float (double-precision)") (InputAction :type "InputAction Object Reference" :default "/Game/Modelo_ARQ/Inputs/IA_Boton_X.IA_Boton_X"))
  ;[0.9819 0.2169 1] Modo Medicion
  (:`Started`
    (if (and ActionValue (`self.M_Medicion`))
      (`self.LimpiarMedicion`))))

(event `EnhancedInput|/Game/Modelo_ARQ/Inputs/IA_Boton_Y`
  (params (ActionValue :type Boolean) (ElapsedSeconds :type "Float (double-precision)") (TriggeredSeconds :type "Float (double-precision)") (InputAction :type "InputAction Object Reference" :default "/Game/Modelo_ARQ/Inputs/IA_Boton_Y.IA_Boton_Y"))
  ;[0.9819 0.2169 1] Modo Medicion
  (:`Started`
    (if (and ActionValue (`self.M_Medicion`))
      (bind _outactors (`GameplayStatics.GetAllActorsOfClass` "/Game/CollaborativeViewer/Blueprints/Commands/Dimension/BPs/BP_Dimenssion.BP_Dimenssion_C"))
      (bind _output (`|GetArrayItem` _outactors (- (`KismetArrayLibrary.Array_Length` _outactors) 1)))
      (`/Engine/EditorBlueprintResources/StandardMacros.IsValid` _output
        (:`Is Valid`
          (`self.K2_DestroyActor` _output))))))

(event `4D_Modo_iniciar`
  ;[1 1 0.11] SIMULACION 4D
  ;;[1 1 1] ocultar modelo
  (bind _outrownames (`DataTableFunctionLibrary.GetDataTableRowNames` "/Game/Modelo_ARQ/DataProject/ParametrosModelo-CasaRural_Feb.ParametrosModelo-CasaRural_Feb"))
  (for _index (range (`KismetArrayLibrary.Array_Length` _outrownames))
    (`self.Hidden/Visible` true _index))
  (set `self.4D_contador` true)
  (set `self.4DTimer` 0.0))

(event `EnhancedInput|/Game/Modelo_ARQ/Inputs/IA_Boton_B`
  (params (ActionValue :type Boolean) (ElapsedSeconds :type "Float (double-precision)") (TriggeredSeconds :type "Float (double-precision)") (InputAction :type "InputAction Object Reference" :default "/Game/Modelo_ARQ/Inputs/IA_Boton_B.IA_Boton_B"))
  ;[1 1 0.11] SIMULACION 4D
  (:`Started`
    (if (and (`self.M_4D`) (`self.4D_contador`))
      (set `self.4DTimer` 0.0)
      (if (<= (stale `TimerClock` _output_get) 48.0) :!label _label_2
        (bind _returnvalue (`DataTableFunctionLibrary.GetDataTableColumnAsString` "/Game/Modelo_ARQ/DataProject/ParametrosModelo-CasaRural_Feb.ParametrosModelo-CasaRural_Feb" "Start"))
        (for _index (range (`KismetArrayLibrary.Array_Length` _returnvalue))
          (`self.Hidden/Visible` (>= (`KismetStringLibrary.Conv_StringToInt` (`|GetArrayItem` _returnvalue _index)) (`KismetMathLibrary.Conv_DoubleToInt64` (stale `TimerClock` _output_get))) _index))
        (else
          (set `self.4D_contador` false)
          (set `self.4DTimer` 0.0))))))

(event `TimerClock`
  ;[1 1 0.11] SIMULACION 4D
  (if (and (`self.M_4D`) (`self.4D_contador`))
    (bind _output_get (set `self.4DTimer` (+ (* (`GameplayStatics.GetWorldDeltaSeconds`) 2.5) (`self.4DTimer`))))
    (goto _label_2)))

(event `EnhancedInput|/Game/Modelo_ARQ/Inputs/IA_Boton_X`
  (params (ActionValue :type Boolean) (ElapsedSeconds :type "Float (double-precision)") (TriggeredSeconds :type "Float (double-precision)") (InputAction :type "InputAction Object Reference" :default "/Game/Modelo_ARQ/Inputs/IA_Boton_X.IA_Boton_X"))
  ;[1 1 0.11] SIMULACION 4D
  (:`Started`
    (if (`self.M_4D`)
      (set `self.4D_contador` false)
      (set `self.4DTimer` 0.0)
      (`self.Aparecer Modelo`))))

(event `Aparecer Modelo`
  ;[1 1 0.11] SIMULACION 4D
  (bind _outrownames (`DataTableFunctionLibrary.GetDataTableRowNames` "/Game/Modelo_ARQ/DataProject/ParametrosModelo-CasaRural_Feb.ParametrosModelo-CasaRural_Feb"))
  (for _index (range (`KismetArrayLibrary.Array_Length` _outrownames))
    (`self.Hidden/Visible` false _index)))

(event `/Game/Modelo_ARQ/Blueprint/BI_Filtro.Lista_Chk`
  (params (Walls :type Boolean) (SFr :type Boolean) (SFo :type Boolean) (SR :type Boolean) (Roof :type Boolean) (Fur :type Boolean) (Win :type Boolean) (Plum :type Boolean) (Floor :type Boolean) (Door :type Boolean))
  ;[1 0.08707 0.3393] Filtro de Visualización
)

(event `Filtro`
  (bind _mask_filtro (`self.Mask Filtro`))
  ;[1 0.08707 0.3393] Filtro de Visualización
  (if (`self.M_Filtro`)
    (bind _array (`|MakeArray` (stale `/Game/Modelo_ARQ/Blueprint/BI_Filtro.Lista_Chk` Walls) (stale `/Game/Modelo_ARQ/Blueprint/BI_Filtro.Lista_Chk` SFr) (stale `/Game/Modelo_ARQ/Blueprint/BI_Filtro.Lista_Chk` SFo) (stale `/Game/Modelo_ARQ/Blueprint/BI_Filtro.Lista_Chk` SR) (stale `/Game/Modelo_ARQ/Blueprint/BI_Filtro.Lista_Chk` Roof) (stale `/Game/Modelo_ARQ/Blueprint/BI_Filtro.Lista_Chk` Fur) (stale `/Game/Modelo_ARQ/Blueprint/BI_Filtro.Lista_Chk` Win) (stale `/Game/Modelo_ARQ/Blueprint/BI_Filtro.Lista_Chk` Plum) (stale `/Game/Modelo_ARQ/Blueprint/BI_Filtro.Lista_Chk` Floor) (stale `/Game/Modelo_ARQ/Blueprint/BI_Filtro.Lista_Chk` Door)))
    (for _index (range (`KismetArrayLibrary.Array_Length` _array))
      (if (not (`|GetArrayItem` _array _index))
        (`KismetArrayLibrary.Array_Add` (`self.Filtro On`) (`|GetArrayItem` (`self.List Filtro`) _index))))
    (set `self.List Filtro` (`self.Filtro On`))
    (`KismetArrayLibrary.Array_Clear` (`self.Filtro On`))
    (bind _returnvalue (`DataTableFunctionLibrary.GetDataTableColumnAsString` "/Game/Modelo_ARQ/DataProject/ParametrosModelo-CasaRural_Feb.ParametrosModelo-CasaRural_Feb" "Category"))
    (for _index_2 (range (`KismetArrayLibrary.Array_Length` _returnvalue))
      (`KismetArrayLibrary.Array_Add` (`self.Mask Filtro`) (`KismetArrayLibrary.Array_Contains` (`self.Filtro On`) (`|GetArrayItem` _returnvalue _index_2))))
    (for _index_3 (range (`KismetArrayLibrary.Array_Length` _mask_filtro))
      (`self.Hidden/Visible` (`|GetArrayItem` _mask_filtro _index_3) _index_3))
    (`KismetArrayLibrary.Array_Clear` (`self.Mask Filtro`))
    (else
      (`KismetArrayLibrary.Array_Clear` (`self.Filtro On`)))))

(event `EnhancedInput|/Game/Modelo_ARQ/Inputs/IA_Disparo_R`
  (params (ActionValue :type Boolean) (ElapsedSeconds :type "Float (double-precision)") (TriggeredSeconds :type "Float (double-precision)") (InputAction :type "InputAction Object Reference" :default "/Game/Modelo_ARQ/Inputs/IA_Disparo_R.IA_Disparo_R"))
  (bind _camera (`self.Camera`))
  (bind (_returnvalue_roll _returnvalue_pitch _returnvalue_yaw) (`KismetMathLibrary.BreakRotator` (`SceneComponent.K2_GetComponentRotation` _camera)))
  ;[0.9062 0.2823 0.01416] Seleccion
  (:`Started`
    (if (`self.M_Seleccion`)
      (bind (_start _end _hitevent) (`self.TrazadoApuntador` (`self.MotionController_R`)))
      (bind (_bblockinghit _binitialoverlap _time _distance _location _impactpoint _normal _impactnormal _physmat _hitactor) (`GameplayStatics.BreakHitResult` _hitevent))
      (if (`KismetStringLibrary.NotEqual_StrStr` (`KismetStringLibrary.Conv_NameToString` (`|GetArrayItem` (`Actor.Tags` _hitactor))))
        (`|ExecutionSequence`
          (:`then_0`
            (bind _outrownames (`DataTableFunctionLibrary.GetDataTableRowNames` "/Game/Modelo_ARQ/DataProject/ParametrosModelo-CasaRural_Feb.ParametrosModelo-CasaRural_Feb"))
            (for _index (range (`KismetArrayLibrary.Array_Length` _outrownames))
              (if (== (`|GetArrayItem` _outrownames _index) "None")
                (bind _returnvalue (`DataTableFunctionLibrary.GetDataTableColumnAsString` "/Game/Modelo_ARQ/DataProject/ParametrosModelo-CasaRural_Feb.ParametrosModelo-CasaRural_Feb" "Assembly Code"))
                (bind _output_get (set `self.Assembly Code` (`|GetArrayItem` _returnvalue _index)))
                (bind _keys (`BlueprintMapLibrary.Map_Keys` (`self.Material`)))
                (set `self.Esp Si` (`KismetArrayLibrary.Array_Contains` _keys _output_get)))))
          (:`then_1`
            (bind _returnvalue_2 (`GameplayStatics.GetActorOfClass` "/Game/Modelo_ARQ/Especificaciones/MP_Plane.MP_Plane_C"))
            (`/Engine/EditorBlueprintResources/StandardMacros.IsValid` _returnvalue_2
              (:`Is Valid`
                (`self.K2_DestroyActor` _returnvalue_2))
              (:`Is Not Valid`
                _))
            (if (`self.Esp Si`)
              (bind (_returnvalue_x _returnvalue_y) (`KismetMathLibrary.BreakVector` (+ (* (- (`SceneComponent.K2_GetComponentLocation` _camera) _location) 0.2) _location)))
              (`|SpawnActorFromClass` "/Game/Modelo_ARQ/Especificaciones/MP_Plane.MP_Plane_C" (`KismetMathLibrary.MakeTransform` (`KismetMathLibrary.MakeVector` _returnvalue_x _returnvalue_y 120.0) (`KismetMathLibrary.MakeRotator` 0.0 0.0 (+ _returnvalue_yaw 90.0))) "Undefined" "MultiplyWithRoot" null null)
              (bind _returnvalue_3 (`GameplayStatics.GetActorOfClass` "/Game/Modelo_ARQ/Especificaciones/MP_Plane.MP_Plane_C"))
              (`PrimitiveComponent.SetMaterial` (`/Game/Modelo_ARQ/Especificaciones/MP_Plane.Plane` _returnvalue_3) 0 (`BlueprintMapLibrary.Map_Find` (`self.Material`) (`self.Assembly Code`)))
              (`self.SetActorEnableCollision` _returnvalue_3 false)
              (set `self.Assembly Code` ""))))
        (else
          (bind _returnvalue_4 (`GameplayStatics.GetActorOfClass` "/Game/Modelo_ARQ/Especificaciones/MP_Plane.MP_Plane_C"))
          (`/Engine/EditorBlueprintResources/StandardMacros.IsValid` _returnvalue_4
            (:`Is Valid`
              (`self.K2_DestroyActor` _returnvalue_4))))))))

(fn `Activa_Menu`
  (returns (ReturnValue :type Boolean))
  (bind _camera (`self.Camera`))
  (bind _arrow1 (`self.Arrow1`))
  (return (and (== (`SceneComponent.GetForwardVector` _arrow1) (`KismetMathLibrary.GetForwardVector` (`KismetMathLibrary.FindLookAtRotation` (`SceneComponent.K2_GetComponentLocation` _arrow1) (`SceneComponent.K2_GetComponentLocation` (`self.Camera`)))) :`ErrorTolerance` (`self.Sensibilidad_menu`)) (== (`SceneComponent.GetForwardVector` _camera) (`KismetMathLibrary.GetForwardVector` (`KismetMathLibrary.FindLookAtRotation` (`SceneComponent.K2_GetComponentLocation` _camera) (`SceneComponent.K2_GetComponentLocation` (`self.Arrow1`)))) :`ErrorTolerance` (- 1.0 (`self.Sensibilidad_menu`))))))

(fn `Hidden/Visible`
  (params (Ocultar :type Boolean) (Index :type Integer))
  (bind _outrownames (`DataTableFunctionLibrary.GetDataTableRowNames` "/Game/Modelo_ARQ/DataProject/ParametrosModelo-CasaRural_Feb.ParametrosModelo-CasaRural_Feb"))
  (bind _outactors (`GameplayStatics.GetAllActorsWithTag` (`|GetArrayItem` _outrownames Index)))
  (bind _output (`|GetArrayItem` _outactors))
  (`self.SetActorHiddenInGame` _output Ocultar)
  (`self.SetActorEnableCollision` _output (not Ocultar)))

(fn `LimpiarMedicion`
  (bind _outactors (`GameplayStatics.GetAllActorsOfClass` "/Game/CollaborativeViewer/Blueprints/Commands/Dimension/BPs/BP_Dimenssion.BP_Dimenssion_C" :!label _label))
  (bind _returnvalue (`KismetArrayLibrary.Array_Length` _outactors))
  (while (!= _returnvalue 0)
    (`self.K2_DestroyActor` (`|GetArrayItem` _outactors (- _returnvalue 1)))
    (goto _label)))

(fn `TrazadoApuntador`
  (params (ControlDominio :type "SceneComponent Object Reference"))
  (returns (Start :type "Vector Structure") (End :type "Vector Structure") (HitEvent :type "HitResult Structure"))
  (bind _returnvalue (`SceneComponent.GetSocketRotation` ControlDominio "Begin"))
  (bind _returnvalue_2 (`SceneComponent.GetSocketLocation` ControlDominio "Begin"))
  (bind _returnvalue_3 (+ _returnvalue_2 (0.0 0.0 0.0)))
  (bind _returnvalue_4 (+ _returnvalue_2 (* (`KismetMathLibrary.RotateAngleAxis` (`KismetMathLibrary.GetForwardVector` _returnvalue) 70.0 (`KismetMathLibrary.GetRightVector` _returnvalue)) 500.0)))
  (bind _outhit (`KismetSystemLibrary.LineTraceSingle` :`Start` _returnvalue_3 :`End` _returnvalue_4 :`TraceChannel` "TraceTypeQuery1" :`bTraceComplex` true :`bIgnoreSelf` false :`TraceColor` (struct :`R` 0.237802 :`G` 0.950225 :`B` 1.0 :`A` 1.0) :`DrawTime` 1.0))
  (return _returnvalue_3 _returnvalue_4 _outhit))

(fn `UserConstructionScript`)